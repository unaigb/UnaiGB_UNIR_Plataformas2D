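; BP_Bullet is a projectile for the 2D platformer weapons that damages objects tagged "Muro".
; Each Tick moves it along its forward vector at Speed, without sweep.
; A Sphere overlap with a tagged actor applies damage and destroys the bullet, while a timer set on BeginPlay destroys it after a short lifetime.
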(event `self.ReceiveBeginPlay`
  (`KismetSystemLibrary.K2_SetTimerDelegate` (delegate `DestroyBullet`) 3.0))

(event `DestroyBullet`
  (`self.K2_DestroyActor`))

(event `self.ReceiveTick`
  (params (DeltaSeconds :type "Float (single-precision)"))
  (`self.K2_SetActorLocation` (+ (`self.K2_GetActorLocation`) (* (* (`self.speed`) DeltaSeconds) (`self.GetActorForwardVector`)))))

(event `self.Sphere.OnComponentBeginOverlap`
  (params (OverlappedComponent :type "PrimitiveComponent Object Reference") (OtherActor :type "Actor Object Reference") (OtherComp :type "PrimitiveComponent Object Reference") (OtherBodyIndex :type Integer) (bFromSweep :type Boolean) (SweepResult :type "HitResult Structure (by ref)"))
  (if (`self.ActorHasTag` OtherActor "Muro")
    (`GameplayStatics.ApplyDamage` OtherActor 5.0)
    (`self.K2_DestroyActor`)))

(fn `UserConstructionScript`)